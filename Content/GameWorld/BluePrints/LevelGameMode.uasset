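; Game mode for a two-player level that spawns a flipbook-based character for each joining player and holds possession until both exist.
; PostLogin spawns player one at the first SpawnLoc actor and player two at the second, setting sprite, scale and player number.
; Once the second character exists, both controllers possess their pawns, widgets are cleared, movement input is enabled and each possession triggers the DialogueBot's Talk.
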(event `self.K2_PostLogin`
  (params (NewPlayer :type "PlayerController Object Reference"))
  (`self.Spawn Player` NewPlayer)
  (`/Engine/EditorBlueprintResources/StandardMacros.IsValid` (`self.NewChar2`)
    (:`Is Valid`
      (`KismetSystemLibrary.PrintString` "SECOND PLAYER JOINED" true true (struct :`G` 1.0 :`B` 0.490144 :`A` 1.0) 60.0)
      (`self.Possess New Character1` (`GameplayStatics.GetPlayerController` 0))
      (`self.Possess New Character2` NewPlayer))
    (:`Is Not Valid`
      (`KismetSystemLibrary.PrintString` "SECOND PLAYER NOT JOINED YET" true true (struct :`R` 1.0 :`B` 0.066736 :`A` 1.0) 60.0))))

(fn `Possess New Character1`
  (params (PlayerC :type "PlayerController Object Reference"))
  (bind _newchar1 (`self.NewChar1`))
  (`Controller.Possess` PlayerC _newchar1)
  (`/Game/GameWorld/BluePrints/NewCharacter.RemoveAllWidgets` _newchar1)
  (`/Game/GameWorld/BluePrints/NewCharacter.SetMoveInputEnabled` _newchar1)
  (bind _outactors (`GameplayStatics.GetAllActorsOfClass` "/Game/GameWorld/BluePrints/DialogueBot.DialogueBot_C"))
  (if (== (`KismetArrayLibrary.Array_Length` _outactors) 0)
    (`KismetSystemLibrary.PrintString` "ADD THE DIALOGUE BOT" true true (struct :`R` 0.856177 :`B` 1.0 :`A` 1.0) 60.0)
    (else
      (`/Game/GameWorld/BluePrints/DialogueBot.Talk` (`|GetArrayItem` _outactors))
      (`KismetSystemLibrary.PrintString` "PLAYER1 POSSESSED" true true (struct :`R` 0.856177 :`B` 1.0 :`A` 1.0) 60.0))))

(fn `Possess New Character2`
  (params (PlayerC :type "PlayerController Object Reference"))
  (bind _newchar2 (`self.NewChar2`))
  (`Controller.Possess` PlayerC _newchar2)
  (`/Game/GameWorld/BluePrints/NewCharacter.RemoveAllWidgets` _newchar2)
  (`/Game/GameWorld/BluePrints/NewCharacter.SetMoveInputEnabled` _newchar2)
  (bind _outactors (`GameplayStatics.GetAllActorsOfClass` "/Game/GameWorld/BluePrints/DialogueBot.DialogueBot_C"))
  (if (== (`KismetArrayLibrary.Array_Length` _outactors) 0)
    (`KismetSystemLibrary.PrintString` "ADD THE DIALOGUE BOT" true true (struct :`R` 0.856177 :`B` 1.0 :`A` 1.0) 60.0)
    (else
      (`/Game/GameWorld/BluePrints/DialogueBot.Talk` (`|GetArrayItem` _outactors))
      (`KismetSystemLibrary.PrintString` "PLAYER1 POSSESSED" true true (struct :`R` 0.856177 :`B` 1.0 :`A` 1.0) 60.0))))

(fn `Spawn Player`
  (params (PlayerController :type "PlayerController Object Reference"))
  (`KismetSystemLibrary.PrintString` "ON POST LOGIN")
  (set `self.Player Controller` PlayerController)
  (`/Engine/EditorBlueprintResources/StandardMacros.IsValid` (`Controller.K2_GetPawn` PlayerController)
    (:`Is Not Valid`
      (bind _outactors (`GameplayStatics.GetAllActorsOfClass` "/Game/GameWorld/BluePrints/SpawnLoc.SpawnLoc_C"))
      (if (`self.P1_Spawned`)
        (bind _returnvalue (`|SpawnActorFromClass` "/Game/GameWorld/BluePrints/NewCharacter.NewCharacter_C" (`self.GetTransform` (`|GetArrayItem` _outactors 1)) "AlwaysSpawn" "OverrideRootScale" null null))
        (bind _sprite (`PaperCharacter.Sprite` _returnvalue))
        (`PaperFlipbookComponent.SetFlipbook` _sprite "/Game/GameWorld/Sprites/Player/P2/Flipbooks/P2_rest.P2_rest")
        (`SceneComponent.SetWorldScale3D` _sprite (0.8 0.8 0.8))
        (set `self.NewChar2` _returnvalue)
        (set `/Game/GameWorld/BluePrints/NewCharacter.PlayerNumber` 2 _returnvalue)
        (`KismetSystemLibrary.PrintString` "PLAYER 2 SPAWNED" true true (struct :`R` 0.026183 :`B` 1.0 :`A` 1.0) 60.0)
        (else
          (bind _returnvalue_2 (`|SpawnActorFromClass` "/Game/GameWorld/BluePrints/NewCharacter.NewCharacter_C" (`self.GetTransform` (`|GetArrayItem` _outactors)) "AlwaysSpawn" "OverrideRootScale" null null))
          (bind _sprite_2 (`PaperCharacter.Sprite` _returnvalue_2))
          (`PaperFlipbookComponent.SetFlipbook` _sprite_2 "/Game/GameWorld/Sprites/Player/P1/Flipbooks/P1-rest.P1-rest")
          (`SceneComponent.SetWorldScale3D` _sprite_2 (0.8 0.8 0.8))
          (set `self.NewChar1` _returnvalue_2)
          (set `/Game/GameWorld/BluePrints/NewCharacter.PlayerNumber` 1 _returnvalue_2)
          (set `self.P1_Spawned` true)
          (`KismetSystemLibrary.PrintString` "PLAYER 1 SPAWNED" true true (struct :`R` 0.026183 :`B` 1.0 :`A` 1.0) 60.0))))))

(fn `UserConstructionScript`)