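; DialogueBot is a Blueprint that shows world-specific dialogue one line at a time, with only the W1 world handled in Talk.
; The first Talk call creates a UIText widget holding a back-reference to the bot and switches to UI-only input; later calls advance the line.
; An empty or out-of-range line removes the widget, restores game input and clears IsOpening, so later conversations use W1 instead of the opening W1OD lines.
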(fn `Helper_IncrementAndTextIsValid`
  (params (W :type "Array of Text"))
  (returns (Ret :type Boolean))
  (bind _result (`/Engine/EditorBlueprintResources/StandardMacros.IncrementInt` (`self.LineNum`))
    (:`  `
      (if (or (>= (`self.LineNum`) (`KismetArrayLibrary.Array_Length` W)) (`KismetTextLibrary.TextIsEmpty` (`|GetArrayItem` W _result)))
        (return false)
        (else
          (return true))))))

(fn `Helper_Reset`
  (bind _uitext (`self.UIText`))
  (set `self.LineNum` 0)
  (`/Engine/EditorBlueprintResources/StandardMacros.IsValid` _uitext
    (:`Is Valid`
      (`Widget.RemoveFromParent` _uitext)
      (set `self.UIText` null)
      (`WidgetBlueprintLibrary.SetInputMode_GameOnly` (`GameplayStatics.GetPlayerController` 0))
      (set `self.isOpening` false))))

(fn `Helper_SetUIText`
  (params (UI :type "/Game/Widgets/UIText Object Reference (by ref)") (W :type "Array of Text (by ref)"))
  (set `TextBlock.Text` (`|GetArrayItem` W (`self.LineNum`)) (`/Game/Widgets/UIText.TargetText` UI)))

(fn `Talk`
  (bind _returnvalue (select `bool` (`self.isOpening`) :`false` (`self.W1`) :`true` (`self.W1_OD`)))
  (switch `/Game/GameWorld/BluePrints/WorldENUM` (`self.WorldNum`)
    (:`NewEnumerator0`
      (`/Engine/EditorBlueprintResources/StandardMacros.IsValid` (`self.UIText`)
        (:`Is Valid`
          (bind _ret (`self.Helper_IncrementAndTextIsValid` _returnvalue))
          (if _ret
            (`self.Helper_SetUIText` (`self.UIText`) _returnvalue)
            (else
              (`self.Helper_Reset`))))
        (:`Is Not Valid`
          (bind _returnvalue_2 (`|CreateWidget` "/Game/Widgets/UIText.UIText_C" (`GameplayStatics.GetPlayerController` 0)))
          (set `/Game/Widgets/UIText.UIRef` self _returnvalue_2)
          (bind _output_get (set `self.UIText` _returnvalue_2))
          (`self.Helper_SetUIText` _output_get _returnvalue)
          (`UserWidget.AddToViewport` _output_get 0)
          (`WidgetBlueprintLibrary.SetInputMode_UIOnlyEx` (`GameplayStatics.GetPlayerController` 0) _returnvalue_2)
          (`KismetSystemLibrary.PrintString` "Hello"))))))

(fn `UserConstructionScript`)