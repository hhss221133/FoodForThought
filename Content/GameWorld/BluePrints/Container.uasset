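; Carryable food container in three sizes that the player can fill, hold, empty and drop or place on an AnswerZone.
; OnRep_ContainerSize sets sprite and scale, and stored food is hidden, attached and shown as a combined colour-and-size sprite.
; E-key functions attach the container to the hand socket, hand food back, or release it by overlap.
; Sprite collision is off while held and returns when a character's overlap ends with the area clear.
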(event `self.ReceiveBeginPlay`
  (set `self.IsHoldingFood` false))

(event `self.ReceiveActorEndOverlap`
  (params (OtherActor :type "Actor Object Reference"))
  (if (`KismetMathLibrary.ClassIsChildOf` (`GameplayStatics.GetObjectClass` OtherActor) "/Game/GameWorld/BluePrints/NewCharacter.NewCharacter_C")
    (if (or (> (`KismetArrayLibrary.Array_Length` (`self.GetOverlappingActors` "/Game/GameWorld/BluePrints/NewCharacter.NewCharacter_C")) 0) (> (`KismetArrayLibrary.Array_Length` (`self.GetOverlappingActors` "/Game/GameWorld/World1/AnswerZone.AnswerZone_C")) 0) (> (`KismetArrayLibrary.Array_Length` (`self.GetOverlappingActors` "Container_C")) 0))
      _
      (elif (`self.IsHoldingFood`)
        (if (not (> (`KismetArrayLibrary.Array_Length` (`self.GetOverlappingActors` "/Game/GameWorld/BluePrints/Food.Food_C")) 1))
          (`PrimitiveComponent.SetCollisionEnabled` (`self.ContainerSprite`) "QueryAndPhysics"))
        (elif (not (> (`KismetArrayLibrary.Array_Length` (`self.GetOverlappingActors` "/Game/GameWorld/BluePrints/Food.Food_C")) 0))
          (`PrimitiveComponent.SetCollisionEnabled` (`self.ContainerSprite`) "QueryAndPhysics"))))))

(fn `AttachContainerToPlayer`
  (params (Char :type "/Game/GameWorld/BluePrints/NewCharacter Object Reference"))
  (`self.K2_AttachToComponent` (`PaperCharacter.Sprite` Char) "PlayerHand" "SnapToTarget" "SnapToTarget" "SnapToTarget")
  (`PrimitiveComponent.SetCollisionEnabled` (`self.ContainerSprite`) "NoCollision")
  (bind _holding_ (`self.CheckIfHoldingFood`))
  (if _holding_
    (`PrimitiveComponent.SetCollisionEnabled` (`/Game/GameWorld/BluePrints/Food.FoodTopSprite` (`self.HeldFood`)) "NoCollision")))

(fn `AttachFoodToContainer`
  (params (FoodToContain :type "/Game/GameWorld/BluePrints/Food Object Reference"))
  (bind _output_get (set `self.HeldFood` FoodToContain))
  (set `self.IsHoldingFood` true)
  (`self.SetActorHiddenInGame` _output_get true)
  (bind _combsprite (`self.GetCombineSprite`))
  (`PaperSpriteComponent.SetSprite` (`self.ContainerSprite`) _combsprite)
  (`self.K2_AttachToComponent` _output_get (`self.ContainerSprite`) "ContainerCenter" "SnapToTarget" "SnapToTarget" "SnapToTarget" true)
  (`PrimitiveComponent.SetCollisionEnabled` (`/Game/GameWorld/BluePrints/Food.BoxCollision` (`self.HeldFood`)) "NoCollision"))

(fn `CheckIfHoldingFood`
  (returns (`Holding?` :type Boolean))
  (if (> (`KismetArrayLibrary.Array_Length` (`self.GetAttachedActors` true)) 0)
    (bind _output_get (set `self.IsHoldingFood` true))
    (return _output_get)
    (else
      (bind _output_get_2 (set `self.IsHoldingFood` false))
      (`PaperSpriteComponent.SetSprite` (`self.ContainerSprite`) (select `bool` (== (`self.ContainerSize`) 1) :`false` (select `bool` (== (`self.ContainerSize`) 2) :`false` "/Game/GameWorld/Sprites/Containers/AllContainers_Sprite_2.AllContainers_Sprite_2" :`true` "/Game/GameWorld/Sprites/Containers/AllContainers_Sprite_1.AllContainers_Sprite_1" :!type "PaperSprite Object Reference") :`true` "/Game/GameWorld/Sprites/Containers/AllContainers_Sprite_0.AllContainers_Sprite_0"))
      (return _output_get_2))))

(fn `GetCombineSprite`
  (returns (CombSprite :type "PaperSprite Object Reference"))
  (bind _containersize (`self.ContainerSize`))
  (switch `int` (`/Game/GameWorld/BluePrints/Food.FoodColour` (`self.HeldFood`))
    (:`1`
      (switch `int` _containersize
        (:`1`
          (return "/Game/GameWorld/Sprites/ContFoodComb/AllCombinations_Sprite_9.AllCombinations_Sprite_9"))
        (:`2`
          (return "/Game/GameWorld/Sprites/ContFoodComb/AllCombinations_Sprite_10.AllCombinations_Sprite_10"))
        (:`3`
          (return "/Game/GameWorld/Sprites/ContFoodComb/AllCombinations_Sprite_11.AllCombinations_Sprite_11"))))
    (:`2`
      (switch `int` _containersize
        (:`1`
          (return "/Game/GameWorld/Sprites/ContFoodComb/AllCombinations_Sprite_0.AllCombinations_Sprite_0"))
        (:`2`
          (return "/Game/GameWorld/Sprites/ContFoodComb/AllCombinations_Sprite_2.AllCombinations_Sprite_2"))
        (:`3`
          (return "/Game/GameWorld/Sprites/ContFoodComb/AllCombinations_Sprite_4.AllCombinations_Sprite_4"))))
    (:`3`
      (switch `int` _containersize
        (:`1`
          (return "/Game/GameWorld/Sprites/ContFoodComb/AllCombinations_Sprite_6.AllCombinations_Sprite_6"))
        (:`2`
          (return "/Game/GameWorld/Sprites/ContFoodComb/AllCombinations_Sprite_7.AllCombinations_Sprite_7"))
        (:`3`
          (return "/Game/GameWorld/Sprites/ContFoodComb/AllCombinations_Sprite_8.AllCombinations_Sprite_8"))))))

(fn `On_E_Held`
  (params (Player :type "/Game/GameWorld/BluePrints/NewCharacter Object Reference"))
  (`self.K2_AttachToComponent` (`PaperCharacter.Sprite` Player) "PlayerHand" "SnapToTarget" "SnapToTarget" "SnapToTarget")
  (`PrimitiveComponent.SetCollisionEnabled` (`self.ContainerSprite`) "NoCollision")
  (bind _holding_ (`self.CheckIfHoldingFood`))
  (if _holding_
    (`PrimitiveComponent.SetCollisionEnabled` (`/Game/GameWorld/BluePrints/Food.FoodTopSprite` (`self.HeldFood`)) "NoCollision")
    (`self.CheckIfHoldingFood`)))

(fn `OnRep_ContainerSize`
  (bind (_returnvalue_location _returnvalue_rotation) (`KismetMathLibrary.BreakTransform` (`self.GetTransform`)))
  (bind (_returnvalue_location_2 _returnvalue_rotation_2) (`KismetMathLibrary.BreakTransform` (`self.GetTransform`)))
  (bind (_returnvalue_location_3 _returnvalue_rotation_3) (`KismetMathLibrary.BreakTransform` (`self.GetTransform`)))
  (bind _returnvalue (`KismetMathLibrary.MakeTransform` _returnvalue_location _returnvalue_rotation (`KismetMathLibrary.MakeVector` 0.2 0.2 0.2)))
  (bind _returnvalue_2 (`KismetMathLibrary.MakeTransform` _returnvalue_location_3 _returnvalue_rotation_3 (`KismetMathLibrary.MakeVector` 0.3 0.3 0.3)))
  (bind _returnvalue_3 (`KismetMathLibrary.MakeTransform` _returnvalue_location_2 _returnvalue_rotation_2 (`KismetMathLibrary.MakeVector` 0.5 0.5 0.5)))
  (if (== (`self.ContainerSize`) 1)
    (`PaperSpriteComponent.SetSprite` (`self.ContainerSprite`) "/Game/GameWorld/Sprites/Containers/AllContainers_Sprite_0.AllContainers_Sprite_0")
    (`self.K2_SetActorTransform` _returnvalue)
    (set `self.InitialScale` _returnvalue)
    (elif (== (`self.ContainerSize`) 2)
      (`PaperSpriteComponent.SetSprite` (`self.ContainerSprite`) "/Game/GameWorld/Sprites/Containers/AllContainers_Sprite_1.AllContainers_Sprite_1")
      (`self.K2_SetActorTransform` _returnvalue_2)
      (set `self.InitialScale` _returnvalue_2)
      (elif (== (`self.ContainerSize`) 3)
        (`PaperSpriteComponent.SetSprite` (`self.ContainerSprite`) "/Game/GameWorld/Sprites/Containers/AllContainers_Sprite_2.AllContainers_Sprite_2")
        (`self.K2_SetActorTransform` _returnvalue_3)
        (set `self.InitialScale` _returnvalue_3)))))

(fn `Post_On_E_Held`
  (params (Player :type "/Game/GameWorld/BluePrints/NewCharacter Object Reference"))
  (locals (TActors :type "Array of Actor Object Reference"))
  (bind (_returnvalue_location _returnvalue_rotation) (`KismetMathLibrary.BreakTransform` (`self.GetTransform`)))
  (bind (_initialscale_location _initialscale_rotation _initialscale_scale) (`KismetMathLibrary.BreakTransform` (`self.InitialScale`)))
  (bind _output_get (set `local.TActors` (`PrimitiveComponent.GetOverlappingActors` (`self.ContainerCollision`) "/Script/Engine.Actor")))
  (`KismetArrayLibrary.Array_RemoveItem` _output_get Player)
  (`KismetArrayLibrary.Array_RemoveItem` _output_get (`self.HeldFood`))
  (if (== (`KismetArrayLibrary.Array_Length` _output_get) 0)
    (`self.K2_DetachFromActor` "KeepWorld" "KeepWorld")
    (`self.K2_SetActorTransform` (`KismetMathLibrary.MakeTransform` _returnvalue_location _returnvalue_rotation _initialscale_scale))
    (else
      (for _array_element (`local.TActors`)
        (if (`KismetMathLibrary.ClassIsChildOf` (`GameplayStatics.GetObjectClass` _array_element) "/Game/GameWorld/World1/AnswerZone.AnswerZone_C")
          (bind _asanswer_zone (cast `/Game/GameWorld/World1/AnswerZone` _array_element))
          (`/Game/GameWorld/World1/AnswerZone.AttachContainerToAnswer` _asanswer_zone self)
          (break))))))

(fn `Pre_E_Interact`
  (params (Player :type "/Game/GameWorld/BluePrints/NewCharacter Object Reference"))
  (bind _heldfood (`self.HeldFood`))
  (bind _holding_ (`self.CheckIfHoldingFood`))
  (if _holding_
    (`/Game/GameWorld/BluePrints/Food.Attach Food to Player` _heldfood Player)
    (`PrimitiveComponent.SetCollisionEnabled` (`/Game/GameWorld/BluePrints/Food.BoxCollision` _heldfood) "QueryAndPhysics")
    (`self.CheckIfHoldingFood`)))

(fn `UserConstructionScript`)