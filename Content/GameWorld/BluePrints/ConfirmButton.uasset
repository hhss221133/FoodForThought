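; ConfirmButton checks the player's answer in a dog-feeding puzzle and offers a reset of all Dog and Food actors.
; With JustMoveNext set, CheckAnswers only requires every Dog to be Correct.
; Otherwise each answer zone needs a container holding food of matching size, and IsAnsArray also requires all containers to be equally sized.
; Reset_FoodAndDog runs only when ResetEnabled is set, finding actors by class.
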(fn `Check All Container Size Equal`
  (returns (`AllEqual?` :type Boolean))
  (set `self.SizeValidator` 0)
  (for _array_element (`self.ButtonAnswerZones`)
    (bind _holding_ (`/Game/GameWorld/World1/AnswerZone.CheckIfHoldingContainer` _array_element))
    (if _holding_
      (if (== (`self.SizeValidator`) 0)
        (bind _containersize (`/Game/GameWorld/BluePrints/Container.ContainerSize` (`/Game/GameWorld/World1/AnswerZone.HeldContainer` _array_element)))
        (set `self.SizeValidator` _containersize)
        (elif (not (== _containersize (`self.SizeValidator`)))
          (return false)))
      (else
        (return false))))
  (return true))

(fn `CheckAllDogsCorrect`
  (returns (CanGoNext :type Boolean))
  (bind _outactors (`GameplayStatics.GetAllActorsOfClass` "/Game/GameWorld/BluePrints/Dog.Dog_C"))
  (for _array_element _outactors
    (if (not (`/Game/GameWorld/BluePrints/Dog.Correct` _array_element))
      (return false)))
  (return true))

(fn `CheckAnswers`
  (returns (`Correct?` :type Boolean))
  (if (`self.JustMoveNext`)
    (bind _cangonext (`self.CheckAllDogsCorrect`))
    (if _cangonext
      (return true)
      (else
        (return false)))
    (else
      (if (`self.IsAnsArray?`)
        (bind _allequal_ (`self.Check All Container Size Equal`))
        (if _allequal_
          _
          (else
            (return false))))
      (set `self.Correct?` true)
      (for _array_element (`self.ButtonAnswerZones`)
        (bind _holding_ (`/Game/GameWorld/World1/AnswerZone.CheckIfHoldingContainer` _array_element))
        (if _holding_
          (bind _heldcontainer (`/Game/GameWorld/World1/AnswerZone.HeldContainer` _array_element))
          (bind _holding__2 (`/Game/GameWorld/BluePrints/Container.CheckIfHoldingFood` _heldcontainer))
          (if _holding__2
            (if (not (== (`/Game/GameWorld/BluePrints/Container.ContainerSize` _heldcontainer) (`/Game/GameWorld/BluePrints/Food.FoodSize` (`/Game/GameWorld/BluePrints/Container.HeldFood` _heldcontainer))))
              (return false))
            (else
              (return false)))
          (else
            (return false))))
      (return (`self.Correct?`)))))

(fn `Reset_FoodAndDog`
  (if (`self.Reset_Enabled`)
    (bind _outactors (`GameplayStatics.GetAllActorsOfClass` "/Game/GameWorld/BluePrints/Dog.Dog_C"))
    (for _array_element _outactors
      (`/Game/GameWorld/BluePrints/Dog.ResetDog` _array_element))
    (bind _outactors_2 (`GameplayStatics.GetAllActorsOfClass` "/Game/GameWorld/BluePrints/Food.Food_C"))
    (for _array_element_2 _outactors_2
      (`/Game/GameWorld/BluePrints/Food.Reset_Food` _array_element_2))))

(fn `UserConstructionScript`)