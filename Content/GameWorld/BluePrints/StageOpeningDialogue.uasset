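; Stage opening dialogue Blueprint that shows the intro text for a world, with only the W1 case handled.
; SOTalk, also called from the Construction Script, creates the UIText widget on first call and advances one line on each later call.
; Helpers bounds-check the line array and set the widget text.
; When lines run out, they reset the index, remove the widget, re-enable NC movement and set its InitialDialogue flag.
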(fn `Helper_IncrementAndTextIsValid`
  (params (W :type "Array of Text"))
  (returns (Ret :type Boolean))
  (bind _result (`/Engine/EditorBlueprintResources/StandardMacros.IncrementInt` (`self.LineNum`))
    (:`  `
      (if (or (>= (`self.LineNum`) (`KismetArrayLibrary.Array_Length` W)) (`KismetTextLibrary.TextIsEmpty` (`|GetArrayItem` W _result)))
        (return false)
        (else
          (return true))))))

(fn `Helper_Reset`
  (params (NC :type "/Game/GameWorld/BluePrints/NewCharacter Object Reference"))
  (set `self.LineNum` 0)
  (`Widget.RemoveFromParent` (`self.UIText`))
  (set `self.UIText` null)
  (set `/Game/GameWorld/BluePrints/NewCharacter.AllowMovement` true NC)
  (set `/Game/GameWorld/BluePrints/NewCharacter.InitialDialogue` true NC))

(fn `Helper_SetUIText`
  (params (UI :type "/Game/Widgets/UIText Object Reference (by ref)") (W :type "Array of Text (by ref)"))
  (set `TextBlock.Text` (`|GetArrayItem` W (`self.LineNum`)) (`/Game/Widgets/UIText.TargetText` UI)))

(fn `S O Talk`
  (params (NC :type "/Game/GameWorld/BluePrints/NewCharacter Object Reference"))
  (bind _w1 (`self.W1`))
  (switch `/Game/GameWorld/BluePrints/WorldENUM` (`self.WorldNum`)
    (:`NewEnumerator0`
      (`/Engine/EditorBlueprintResources/StandardMacros.IsValid` (`self.UIText`)
        (:`Is Valid`
          (bind _ret (`self.Helper_IncrementAndTextIsValid` _w1))
          (if _ret
            (`self.Helper_SetUIText` (`self.UIText`) _w1)
            (else
              (`self.Helper_Reset` NC))))
        (:`Is Not Valid`
          (bind _returnvalue (`|CreateWidget` "/Game/Widgets/UIText.UIText_C" (`GameplayStatics.GetPlayerController` 0)))
          (bind _output_get (set `self.UIText` _returnvalue))
          (`self.Helper_SetUIText` _output_get _w1)
          (`UserWidget.AddToViewport` _output_get 0))))))

(fn `UserConstructionScript`
  (`self.S O Talk` null))