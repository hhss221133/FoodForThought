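; Dog actor that reacts to being fed a food item in what appears to be a food-matching game.
; Get Fed compares the food's colour and size against the dog's ColorNeed and SizeNeed.
; The dog sprite tints green when both match and red otherwise, and IsFed becomes true in either case.
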(fn `Get Fed`
  (params (Food :type "/Game/GameWorld/BluePrints/Food Object Reference"))
  (if (and (== (`/Game/GameWorld/BluePrints/Food.FoodColour` Food) (`self.ColorNeed`)) (== (`/Game/GameWorld/BluePrints/Food.FoodSize` Food) (`self.SizeNeed`)))
    (`PaperSpriteComponent.SetSpriteColor` (`self.DogSprite`) (struct :`G` 0.562 :`A` 1.0))
    (set `self.IsFed?` true)
    (else
      (`PaperSpriteComponent.SetSpriteColor` (`self.DogSprite`) (struct :`R` 0.562 :`B` 0.069378 :`A` 1.0))
      (set `self.IsFed?` true))))

(fn `UserConstructionScript`)