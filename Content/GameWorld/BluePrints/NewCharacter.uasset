(event `InputAction|Interact`
  (params (Key :type "Key Structure"))
  (bind _overlappingactors (`self.GetOverlappingActors` "/Game/GameWorld/BluePrints/Container.Container_C"))
  (bind _overlappingactors_2 (`self.GetOverlappingActors` "/Game/GameWorld/World1/AnswerZone.AnswerZone_C"))
  (bind _overlappingactors_3 (`self.GetOverlappingActors` "/Game/GameWorld/World1/ConfirmButton.ConfirmButton_C"))
  (bind _overlappingactors_4 (`self.GetOverlappingActors` "/Game/GameWorld/BluePrints/Food.Food_C"))
  (bind _heldcontainer (`self.HeldContainer`))
  (bind _heldfood (`self.HeldFood`))
  (bind _heldcontainer_2 (`self.HeldContainer`))
  (bind _heldfood_2 (`self.HeldFood`))
  (bind (_returnvalue_location _returnvalue_rotation) (`KismetMathLibrary.BreakTransform` (`self.GetTransform` _heldcontainer_2)))
  (bind (_returnvalue_location_2 _returnvalue_rotation_2) (`KismetMathLibrary.BreakTransform` (`self.GetTransform` _heldfood_2)))
  (bind (_initialscale_location _initialscale_rotation _initialscale_scale) (`KismetMathLibrary.BreakTransform` (`/Game/GameWorld/BluePrints/Container.InitialScale` _heldcontainer_2)))
  (bind (_initialscale_location_2 _initialscale_rotation_2 _initialscale_scale_2) (`KismetMathLibrary.BreakTransform` (`/Game/GameWorld/BluePrints/Food.InitialScale` _heldfood_2)))
  (bind _returnvalue (`KismetArrayLibrary.Array_Length` (`self.GetAttachedActors` (`self.HeldContainer`) true false)))
  ;[1 1 1] Detect Short or Long "E" press
  (:`Pressed`
    (set `self.IsKeyHeld` false)
    (`KismetSystemLibrary.RetriggerableDelay` 0.3)
    (set `self.IsKeyHeld` true))
  (:`Released`
    (if (`self.IsKeyHeld`)
      (if (`self.PlayerIsHoldingFood`)
        (`KismetSystemLibrary.PrintString` "Hello")
        (elif (`self.PlayerIsHoldingContainer`)
          (if (== (`KismetArrayLibrary.Array_Length` _overlappingactors_2) 0)
            ;[1 1 1] Put down container to empty space
            (if (or (== _returnvalue 0) (== _returnvalue 1))
              (if (== (`KismetArrayLibrary.Array_Length` (`self.GetOverlappingActors` "/Script/Engine.Actor")) (+ _returnvalue 1))
                (`self.Play Pickup Sound`)
                (`/Engine/EditorBlueprintResources/ActorMacros.Switch Has Authority`
                  (:`Authority`
                    (`self.PutDownContainer`))
                  (:`Remote`
                    (`self.K2_DetachFromActor` _heldcontainer_2 "KeepWorld" "KeepWorld" "KeepRelative")
                    (set `self.PlayerIsHoldingContainer` false)
                    (`self.K2_SetActorTransform` _heldcontainer_2 (`KismetMathLibrary.MakeTransform` _returnvalue_location _returnvalue_rotation _initialscale_scale) false false)
                    (`self.ClientPutDownContainer`)))))
            (else
              ;[1 1 1] Attach container to answer
              (`self.Play Pickup Sound`)
              (bind _asanswer_zone (cast `/Game/GameWorld/World1/AnswerZone` (`|GetArrayItem` _overlappingactors_2)))
              (`/Engine/EditorBlueprintResources/ActorMacros.Switch Has Authority`
                (:`Authority`
                  (`/Game/GameWorld/World1/AnswerZone.MulticastAttachFoodToAnswer` _asanswer_zone (`self.HeldContainer`) self))
                (:`Remote`
                  (set `self.PlayerIsHoldingContainer` false)
                  (`/Game/GameWorld/World1/AnswerZone.AttachContainerToAnswer` _asanswer_zone _heldcontainer)
                  (`self.ClientAttachContainerToAnswer` _asanswer_zone _heldcontainer)))))
          (else
            ;[1 1 1] Pickup container
            (if (> (`KismetArrayLibrary.Array_Length` _overlappingactors) 0)
              (bind _ascontainer (cast `/Game/GameWorld/BluePrints/Container` (`|GetArrayItem` _overlappingactors)))
              (`self.Play Pickup Sound`)
              (`/Engine/EditorBlueprintResources/ActorMacros.Switch Has Authority`
                (:`Authority`
                  (`self.PickupContainer` _ascontainer))
                (:`Remote`
                  (bind _output_get (set `self.HeldContainer` _ascontainer))
                  (set `self.PlayerIsHoldingContainer` true)
                  (`/Game/GameWorld/BluePrints/Container.AttachContainerToPlayer` _output_get self)
                  (`self.ClientPickupContainer` _output_get)))))))
      (elif (`self.PlayerIsHoldingFood`)
        (bind (_actor _actorenum) (`self.GetNearActors` (`self.HeldFood`)))
        (switch `/Game/GameWorld/BluePrints/ActorTypes` _actorenum
          (:`NewEnumerator1`
            ;[1 1 1] Put food into container
            (if (== (`KismetArrayLibrary.Array_Length` (`self.GetAttachedActors` _actor true false)) 0)
              (bind _ascontainer_2 (cast `/Game/GameWorld/BluePrints/Container` _actor))
              (`self.Play Pickup Sound`)
              (`/Engine/EditorBlueprintResources/ActorMacros.Switch Has Authority`
                (:`Authority`
                  (`self.FoodIntoContainer` _ascontainer_2))
                (:`Remote`
                  (set `self.PlayerIsHoldingFood` false)
                  (`/Game/GameWorld/BluePrints/Container.AttachFoodToContainer` _ascontainer_2 (`self.HeldFood`))
                  (`self.ClientFoodIntoContainer` _ascontainer_2)))))
          (:`NewEnumerator4`
            (bind _asdog (cast `/Game/GameWorld/BluePrints/Dog` _actor))
            (`self.FeedFoodToDog` _asdog (`self.HeldFood`)))
          (:`NewEnumerator6`
            ;[1 1 1] Put down food to empty space
            (`self.Play Pickup Sound`)
            (`/Engine/EditorBlueprintResources/ActorMacros.Switch Has Authority`
              (:`Authority`
                (`self.PutDownFood`))
              (:`Remote`
                (`self.K2_DetachFromActor` _heldfood_2 "KeepWorld" "KeepWorld" "KeepRelative")
                (set `self.PlayerIsHoldingFood` false)
                (`self.K2_SetActorTransform` _heldfood_2 (`KismetMathLibrary.MakeTransform` _returnvalue_location_2 _returnvalue_rotation_2 _initialscale_scale_2) false false)
                (`self.ClientPutDownFood`))))
          (:`NewEnumerator7`
            ;[1 1 1] Put food into branch
            (if (== (`KismetArrayLibrary.Array_Length` (`self.GetAttachedActors` _actor true false)) 0)
              (bind _asbranch_select (cast `/Game/GameWorld/World2/BranchSelect` _actor))
              (`self.Play Pickup Sound`)
              (`/Engine/EditorBlueprintResources/ActorMacros.Switch Has Authority`
                (:`Authority`
                  (`self.FoodIntoBranch` _asbranch_select)
                  (`KismetSystemLibrary.RetriggerableDelay` 2.0)
                  (`self.CheckingLeftOrRight` _asbranch_select _heldfood))
                (:`Remote`
                  (set `self.PlayerIsHoldingFood` false)
                  (`/Game/GameWorld/World2/BranchSelect.AttachFoodToBranch` _asbranch_select _heldfood)
                  (`self.ClientFoodIntoBranch` _asbranch_select)
                  (`KismetSystemLibrary.RetriggerableDelay` 2.0)
                  (`/Game/GameWorld/World2/BranchSelect.BranchLeftOrRight` _asbranch_select _heldfood)
                  (`self.ClientCheckingLeftOrRight` _asbranch_select _heldfood))))))
        (elif (`self.PlayerIsHoldingContainer`)
          _
          (elif (> (`KismetArrayLibrary.Array_Length` _overlappingactors_3) 0)
            ;[1 1 1] Confirm button check answers
            (bind _asconfirm_button (cast `/Game/GameWorld/World1/ConfirmButton` (`|GetArrayItem` _overlappingactors_3)))
            (bind _correct_ (`/Game/GameWorld/World1/ConfirmButton.CheckAnswers` _asconfirm_button))
            (if _correct_
              (`/Engine/EditorBlueprintResources/ActorMacros.Switch Has Authority`
                (:`Authority`
                  (bind _nextstage (`/Game/GameWorld/World1/ConfirmButton.NextStage` _asconfirm_button))
                  (`self.Next level` _nextstage))
                (:`Remote`
                  (bind _returnvalue_2 (`|CreateWidget` "/Game/LoadingScreen/LoadingScreenWidget.LoadingScreenWidget_C"))
                  (`UserWidget.AddToViewport` _returnvalue_2 1)
                  (`self.Next level` _nextstage)))
              (else
                (`KismetSystemLibrary.PrintString` "INCORRECT")))
            (else
              ;[1 1 1] Pickup Food no container around
              (if (> (`KismetArrayLibrary.Array_Length` _overlappingactors_4) 0)
                (bind _asfood (cast `/Game/GameWorld/BluePrints/Food` (`|GetArrayItem` _overlappingactors_4)))
                (`self.Play Pickup Sound`)
                (bind _returnvalue_3 (`self.GetAttachParentActor` _asfood))
                (`/Engine/EditorBlueprintResources/StandardMacros.IsValid` _returnvalue_3
                  (:`Is Valid`
                    ;[1 1 1] Pickup food from container
                    (if (`KismetMathLibrary.ClassIsChildOf` (`GameplayStatics.GetObjectClass` _returnvalue_3) "/Game/GameWorld/BluePrints/Container.Container_C")
                      (bind _ascontainer_3 (cast `/Game/GameWorld/BluePrints/Container` _returnvalue_3))
                      (`/Engine/EditorBlueprintResources/ActorMacros.Switch Has Authority`
                        (:`Authority`
                          (`self.PickupFood` _asfood)
                          (`self.UpdateContainer` _ascontainer_3))
                        (:`Remote`
                          (bind _output_get_2 (set `self.HeldFood` _asfood))
                          (set `self.PlayerIsHoldingFood` true)
                          (`/Game/GameWorld/BluePrints/Food.Attach Food to Player` _output_get_2 self)
                          (`self.ClientPickupFood` (`self.HeldFood`))
                          (`/Game/GameWorld/BluePrints/Container.CheckIfHoldingFood` _ascontainer_3)
                          (`self.ClientUpdateContainer` _ascontainer_3)))))
                  (:`Is Not Valid`
                    (`/Engine/EditorBlueprintResources/ActorMacros.Switch Has Authority`
                      (:`Authority`
                        (`self.PickupFood` _asfood))
                      (:`Remote`
                        (bind _output_get_3 (set `self.HeldFood` _asfood))
                        (set `self.PlayerIsHoldingFood` true)
                        (`/Game/GameWorld/BluePrints/Food.Attach Food to Player` _output_get_3 self)
                        (`self.ClientPickupFood` (`self.HeldFood`))))))))))))))

(event `PickupFood`
  (params (Food :type "/Game/GameWorld/BluePrints/Food Object Reference"))
  ;[1 1 1] Pick Up Food
  (bind _output_get (set `self.HeldFood` Food))
  (set `self.PlayerIsHoldingFood` true)
  (`/Game/GameWorld/BluePrints/Food.Attach Food to Player` _output_get self))

(event `FoodIntoContainer`
  (params (Container :type "/Game/GameWorld/BluePrints/Container Object Reference"))
  ;[1 1 1] Food Into Container
  (set `self.PlayerIsHoldingFood` false)
  (`/Game/GameWorld/BluePrints/Container.AttachFoodToContainer` Container (`self.HeldFood`)))

(event `PutDownFood`
  (bind _heldfood (`self.HeldFood`))
  (bind (_returnvalue_location _returnvalue_rotation) (`KismetMathLibrary.BreakTransform` (`self.GetTransform` _heldfood)))
  (bind (_initialscale_location _initialscale_rotation _initialscale_scale) (`KismetMathLibrary.BreakTransform` (`/Game/GameWorld/BluePrints/Food.InitialScale` _heldfood)))
  ;[1 1 1] Put Food Down
  (`self.K2_DetachFromActor` _heldfood "KeepWorld" "KeepWorld" "KeepRelative")
  (set `self.PlayerIsHoldingFood` false)
  (`self.K2_SetActorTransform` _heldfood (`KismetMathLibrary.MakeTransform` _returnvalue_location _returnvalue_rotation _initialscale_scale) false false))

(event `PickupContainer`
  (params (Container :type "/Game/GameWorld/BluePrints/Container Object Reference"))
  ;[1 1 1] Pick Up Container
  (bind _output_get (set `self.HeldContainer` Container))
  (set `self.PlayerIsHoldingContainer` true)
  (`/Game/GameWorld/BluePrints/Container.AttachContainerToPlayer` _output_get self))

(event `PutDownContainer`
  (bind _heldcontainer (`self.HeldContainer`))
  (bind (_returnvalue_location _returnvalue_rotation) (`KismetMathLibrary.BreakTransform` (`self.GetTransform` _heldcontainer)))
  (bind (_initialscale_location _initialscale_rotation _initialscale_scale) (`KismetMathLibrary.BreakTransform` (`/Game/GameWorld/BluePrints/Container.InitialScale` _heldcontainer)))
  ;[1 1 1] Put Down Container
  (`self.K2_DetachFromActor` _heldcontainer "KeepWorld" "KeepWorld" "KeepRelative")
  (set `self.PlayerIsHoldingContainer` false)
  (`self.K2_SetActorTransform` _heldcontainer (`KismetMathLibrary.MakeTransform` _returnvalue_location _returnvalue_rotation _initialscale_scale) false false))

(event `CycleSize`
  (params (Branch :type "/Game/GameWorld/World2/BranchSelect Object Reference"))
  ;[1 1 1] Cycle branch select size
  (`/Game/GameWorld/World2/BranchSelect.CycleSize` Branch))

(event `SwitchLR`
  (params (Branch :type "/Game/GameWorld/World2/BranchSelect Object Reference"))
  ;[1 1 1] SwitchLR
  (`/Game/GameWorld/World2/BranchSelect.SwitchLR` Branch))

(event `FeedDog`
  (params (Dog :type "/Game/GameWorld/BluePrints/Dog Object Reference") (Food :type "/Game/GameWorld/BluePrints/Food Object Reference"))
  (set `self.PlayerIsHoldingFood` false)
  (`/Game/GameWorld/BluePrints/Dog.Get Fed` Dog Food))

(event `CheckingLeftOrRight`
  (params (BranchSelect :type "/Game/GameWorld/World2/BranchSelect Object Reference") (Food :type "/Game/GameWorld/BluePrints/Food Object Reference"))
  (`/Game/GameWorld/World2/BranchSelect.BranchLeftOrRight` BranchSelect Food))

(event `UpdateContainer`
  (params (Cont :type "/Game/GameWorld/BluePrints/Container Object Reference"))
  (`/Game/GameWorld/BluePrints/Container.CheckIfHoldingFood` Cont))

(event `FoodIntoBranch`
  (params (BranchSelect :type "/Game/GameWorld/World2/BranchSelect Object Reference"))
  ;[1 1 1] Food Into Branch
  (set `self.PlayerIsHoldingFood` false)
  (`/Game/GameWorld/World2/BranchSelect.AttachFoodToBranch` BranchSelect (`self.HeldFood`)))

(event `ClientPickupFood`
  (params (Food :type "/Game/GameWorld/BluePrints/Food Object Reference"))
  ;[1 1 1] Pick Up Food
  (bind _output_get (set `self.HeldFood` Food))
  (set `self.PlayerIsHoldingFood` true)
  (`/Game/GameWorld/BluePrints/Food.Attach Food to Player` _output_get self))

(event `ClientFoodIntoContainer`
  (params (Container :type "/Game/GameWorld/BluePrints/Container Object Reference"))
  ;[1 1 1] Food Into Container
  (set `self.PlayerIsHoldingFood` false)
  (`/Game/GameWorld/BluePrints/Container.AttachFoodToContainer` Container (`self.HeldFood`)))

(event `ClientPutDownFood`
  (bind _heldfood (`self.HeldFood`))
  (bind (_returnvalue_location _returnvalue_rotation) (`KismetMathLibrary.BreakTransform` (`self.GetTransform` _heldfood)))
  (bind (_initialscale_location _initialscale_rotation _initialscale_scale) (`KismetMathLibrary.BreakTransform` (`/Game/GameWorld/BluePrints/Food.InitialScale` _heldfood)))
  ;[1 1 1] Put Food Down
  (`self.K2_DetachFromActor` _heldfood "KeepWorld" "KeepWorld" "KeepRelative")
  (set `self.PlayerIsHoldingFood` false)
  (`self.K2_SetActorTransform` _heldfood (`KismetMathLibrary.MakeTransform` _returnvalue_location _returnvalue_rotation _initialscale_scale) false false))

(event `ClientPickupContainer`
  (params (Container :type "/Game/GameWorld/BluePrints/Container Object Reference"))
  ;[1 1 1] Pick Up Container
  (bind _output_get (set `self.HeldContainer` Container))
  (set `self.PlayerIsHoldingContainer` true)
  (`/Game/GameWorld/BluePrints/Container.AttachContainerToPlayer` _output_get self))

(event `ClientPutDownContainer`
  (bind _heldcontainer (`self.HeldContainer`))
  (bind (_returnvalue_location _returnvalue_rotation) (`KismetMathLibrary.BreakTransform` (`self.GetTransform` _heldcontainer)))
  (bind (_initialscale_location _initialscale_rotation _initialscale_scale) (`KismetMathLibrary.BreakTransform` (`/Game/GameWorld/BluePrints/Container.InitialScale` _heldcontainer)))
  ;[1 1 1] Put Down Container
  (`self.K2_DetachFromActor` _heldcontainer "KeepWorld" "KeepWorld" "KeepRelative")
  (set `self.PlayerIsHoldingContainer` false)
  (`self.K2_SetActorTransform` _heldcontainer (`KismetMathLibrary.MakeTransform` _returnvalue_location _returnvalue_rotation _initialscale_scale) false false))

(event `ClientAttachContainerToAnswer`
  (params (AnswerZone :type "/Game/GameWorld/World1/AnswerZone Object Reference") (Cont :type "/Game/GameWorld/BluePrints/Container Object Reference"))
  ;[1 1 1] Attach container to answer
  (set `self.PlayerIsHoldingContainer` false)
  (`/Game/GameWorld/World1/AnswerZone.AttachContainerToAnswer` AnswerZone Cont))

(event `ClientCycleSize`
  (params (Branch :type "/Game/GameWorld/World2/BranchSelect Object Reference"))
  ;[1 1 1] Cycle branch select size
  (`/Game/GameWorld/World2/BranchSelect.CycleSize` Branch))

(event `ClientSwitchLR`
  (params (Branch :type "/Game/GameWorld/World2/BranchSelect Object Reference"))
  ;[1 1 1] SwitchLR
  (`/Game/GameWorld/World2/BranchSelect.SwitchLR` Branch))

(event `ClientFeedDog`
  (params (Dog :type "/Game/GameWorld/BluePrints/Dog Object Reference") (Food :type "/Game/GameWorld/BluePrints/Food Object Reference"))
  (set `self.PlayerIsHoldingFood` false)
  (`/Game/GameWorld/BluePrints/Dog.Get Fed` Dog Food))

(event `ClientUpdateContainer`
  (params (Cont :type "/Game/GameWorld/BluePrints/Container Object Reference"))
  (`/Game/GameWorld/BluePrints/Container.CheckIfHoldingFood` Cont))

(event `ClientCheckingLeftOrRight`
  (params (BranchSelect :type "/Game/GameWorld/World2/BranchSelect Object Reference") (Food :type "/Game/GameWorld/BluePrints/Food Object Reference"))
  (`/Game/GameWorld/World2/BranchSelect.BranchLeftOrRight` BranchSelect Food))

(event `ClientFoodIntoBranch`
  (params (BranchSelect :type "/Game/GameWorld/World2/BranchSelect Object Reference"))
  ;[1 1 1] Food Into Branch
  (set `self.PlayerIsHoldingFood` false)
  (`/Game/GameWorld/World2/BranchSelect.AttachFoodToBranch` BranchSelect (`self.HeldFood`)))

(event `Play Pickup Sound`
  (`GameplayStatics.PlaySound2D` "/Game/Music/ItemPickup.ItemPickup" 1.0 1.0 0.0 null null))

(event `InputAction|BranchInteract`
  (params (Key :type "Key Structure"))
  (:`Pressed`
    (set `self.IsKeyHeld` false)
    (`KismetSystemLibrary.RetriggerableDelay` 0.3)
    (set `self.IsKeyHeld` true))
  (:`Released`
    (if (`self.IsKeyHeld`)
      ;[1 1 1] Change LR on BranchSelect
      (bind (_result _branchactor) (`self.CheckBranchOverlap`))
      (if _result
        (`self.Play Pickup Sound`)
        (`/Engine/EditorBlueprintResources/ActorMacros.Switch Has Authority`
          (:`Authority`
            (`self.SwitchLR` _branchactor))
          (:`Remote`
            (`/Game/GameWorld/World2/BranchSelect.SwitchLR` _branchactor)
            (`self.ClientSwitchLR` _branchactor))))
      (else
        ;[1 1 1] Change size on BranchSelect
        (bind (_result_2 _branchactor_2) (`self.CheckBranchOverlap`))
        (if _result_2
          (`self.Play Pickup Sound`)
          (`/Engine/EditorBlueprintResources/ActorMacros.Switch Has Authority`
            (:`Authority`
              (`self.CycleSize` _branchactor_2))
            (:`Remote`
              (`/Game/GameWorld/World2/BranchSelect.CycleSize` _branchactor_2)
              (`self.ClientCycleSize` _branchactor_2))))))))

(event `MultiSetFB`
  (`self.SetFlipBook` false))

(event `InputAxis|UpOrDown`
  (params (AxisValue :type "Float (single-precision)"))
  (`self.AddMovementInput` (0.0 0.0 1.0) AxisValue)
  (`/Engine/EditorBlueprintResources/ActorMacros.Switch Has Authority` :!label _label
    (:`Authority`
      (`self.MultiSetFB`))
    (:`Remote`
      (bind _newmovedir (`self.SetFlipBook` false))
      (`KismetSystemLibrary.Delay` 0.2)
      (`self.AnimationROS` _newmovedir))))

(event `InputAxis|LeftOrRight`
  (params (AxisValue :type "Float (single-precision)"))
  (`self.AddMovementInput` (1.0 0.0 0.0) AxisValue)
  (goto _label))

(event `AnimationROS`
  (params (NewParam :type "/Game/GameWorld/BluePrints/MovementDirections Enum" :default "NewEnumerator0"))
  (`self.SetFlipBook` true NewParam))

(event `Next level`
  (params (NextStage :type String))
  (`self.MultiWidget`)
  (`KismetSystemLibrary.ExecuteConsoleCommand` (`KismetStringLibrary.Concat_StrStr` "servertravel " NextStage) null))

(event `MultiWidget`
  (bind _returnvalue (`|CreateWidget` "/Game/LoadingScreen/LoadingScreenWidget.LoadingScreenWidget_C"))
  (`UserWidget.AddToViewport` _returnvalue 1))

(fn `CheckBranchOverlap`
  (returns (Result :type Boolean) (BranchActor :type "/Game/GameWorld/World2/BranchSelect Object Reference"))
  (bind _overlappingactors (`self.GetOverlappingActors` "/Game/GameWorld/World2/BranchSelect.BranchSelect_C"))
  (bind _returnvalue (> (`KismetArrayLibrary.Array_Length` _overlappingactors) 0))
  (if _returnvalue
    (bind _asbranch_select (cast `/Game/GameWorld/World2/BranchSelect` (`|GetArrayItem` _overlappingactors)))
    (return _returnvalue _asbranch_select)
    (else
      (return false null))))

(fn `FeedFoodToDog`
  (params (Dog :type "/Game/GameWorld/BluePrints/Dog Object Reference") (Food :type "/Game/GameWorld/BluePrints/Food Object Reference"))
  (`self.Play Pickup Sound`)
  (`/Engine/EditorBlueprintResources/ActorMacros.Switch Has Authority`
    (:`Authority`
      (`self.FeedDog` Dog Food))
    (:`Remote`
      (`/Game/GameWorld/BluePrints/Dog.Get Fed` Dog Food)
      (set `self.PlayerIsHoldingFood` false)
      (`self.ClientFeedDog` Dog Food))))

(fn `GetNearActors`
  (params (ToCheck :type "Actor Object Reference"))
  (returns (Actor :type "Actor Object Reference") (ActorEnum :type "/Game/GameWorld/BluePrints/ActorTypes Enum"))
  (bind _tempactor (`self.TempActor`))
  (for _array_element (`self.GetOverlappingActors` ToCheck "/Script/Engine.Actor")
    (set `self.TempActor` null)
    (if (not (`KismetMathLibrary.ClassIsChildOf` (`GameplayStatics.GetObjectClass` _array_element) "NewCharacter_C"))
      (bind _output_get (set `self.TempActor` _array_element))
      (bind _returnvalue (`GameplayStatics.GetObjectClass` _output_get))
      (if (`KismetMathLibrary.ClassIsChildOf` _returnvalue "/Game/GameWorld/BluePrints/Food.Food_C")
        (return _tempactor "NewEnumerator0")
        (elif (`KismetMathLibrary.ClassIsChildOf` _returnvalue "/Game/GameWorld/BluePrints/Container.Container_C")
          (return _tempactor "NewEnumerator1")
          (elif (`KismetMathLibrary.ClassIsChildOf` _returnvalue "/Game/GameWorld/World1/AnswerZone.AnswerZone_C")
            (return _tempactor "NewEnumerator2")
            (elif (`KismetMathLibrary.ClassIsChildOf` _returnvalue "/Game/GameWorld/World1/ConfirmButton.ConfirmButton_C")
              (return _tempactor "NewEnumerator3")
              (elif (`KismetMathLibrary.ClassIsChildOf` _returnvalue "/Game/GameWorld/BluePrints/Dog.Dog_C")
                (return _tempactor "NewEnumerator4")
                (elif (`KismetMathLibrary.ClassIsChildOf` _returnvalue "/Game/GameWorld/World2/BranchSelect.BranchSelect_C")
                  (return _tempactor "NewEnumerator7")
                  (else
                    (return null "NewEnumerator6"))))))))))
  (return null "NewEnumerator6"))

(fn `SetFlipBook`
  (params (Client :type Boolean) (MoveDir :type "/Game/GameWorld/BluePrints/MovementDirections Enum" :default "NewEnumerator0"))
  (returns (NewMoveDir :type "/Game/GameWorld/BluePrints/MovementDirections Enum"))
  (bind _lastdirection (`self.LastDirection`))
  (bind _returnvalue (== (`self.PlayerNumber`) 2))
  (if Client
    (set `self.LastDirection` MoveDir)
    (elif (or (!= (`self.GetInputAxisValue`) 0.0) (!= (`self.GetInputAxisValue`) 0.0))
      (set `self.LastDirection` (select `bool` (> (`self.GetInputAxisValue`) 0.0) :`false` (select `bool` (< (`self.GetInputAxisValue`) 0.0) :`false` (select `bool` (> (`self.GetInputAxisValue`) 0.0) :`false` "NewEnumerator2" :`true` "NewEnumerator3" :!type "/Game/GameWorld/BluePrints/MovementDirections Enum") :`true` "NewEnumerator1") :`true` "NewEnumerator0"))))
  (`PaperFlipbookComponent.SetFlipbook` (`self.Sprite`) (select `bool` (> (`KismetMathLibrary.VSize` (`self.GetVelocity`)) 0.0) :`false` (select `/Game/GameWorld/BluePrints/MovementDirections` _lastdirection :`NewEnumerator0` (select `bool` _returnvalue :`false` "/Game/GameWorld/Sprites/Player/P1/Flipbooks/P1_brest.P1_brest" :`true` "/Game/GameWorld/Sprites/Player/P2/Flipbooks/P2_brest.P2_brest" :!type "PaperFlipbook Object Reference") :`NewEnumerator1` (select `bool` _returnvalue :`false` "/Game/GameWorld/Sprites/Player/P1/Flipbooks/P1-rest.P1-rest" :`true` "/Game/GameWorld/Sprites/Player/P2/Flipbooks/P2_rest.P2_rest" :!type "PaperFlipbook Object Reference") :`NewEnumerator2` (select `bool` _returnvalue :`false` "/Game/GameWorld/Sprites/Player/P1/Flipbooks/P1_lrest.P1_lrest" :`true` "/Game/GameWorld/Sprites/Player/P2/Flipbooks/P2_lrest.P2_lrest" :!type "PaperFlipbook Object Reference") :`NewEnumerator3` (select `bool` _returnvalue :`false` "/Game/GameWorld/Sprites/Player/P1/Flipbooks/P1-rest.P1-rest" :`true` "/Game/GameWorld/Sprites/Player/P2/Flipbooks/P2_rest.P2_rest" :!type "PaperFlipbook Object Reference")) :`true` (select `/Game/GameWorld/BluePrints/MovementDirections` _lastdirection :`NewEnumerator0` (select `bool` _returnvalue :`false` "/Game/GameWorld/Sprites/Player/P1/Flipbooks/P1_walk_back.P1_walk_back" :`true` "/Game/GameWorld/Sprites/Player/P2/Flipbooks/P2_walk_back.P2_walk_back" :!type "PaperFlipbook Object Reference") :`NewEnumerator1` (select `bool` _returnvalue :`false` "/Game/GameWorld/Sprites/Player/P1/Flipbooks/P1_walk_front.P1_walk_front" :`true` "/Game/GameWorld/Sprites/Player/P2/Flipbooks/P2_walk_front.P2_walk_front" :!type "PaperFlipbook Object Reference") :`NewEnumerator2` (select `bool` _returnvalue :`false` "/Game/GameWorld/Sprites/Player/P1/Flipbooks/P1_walk_left.P1_walk_left" :`true` "/Game/GameWorld/Sprites/Player/P2/Flipbooks/P2_walk_left.P2_walk_left" :!type "PaperFlipbook Object Reference") :`NewEnumerator3` (select `bool` _returnvalue :`false` "/Game/GameWorld/Sprites/Player/P1/Flipbooks/P1_walk_right.P1_walk_right" :`true` "/Game/GameWorld/Sprites/Player/P2/Flipbooks/P2_walk_right.P2_walk_right" :!type "PaperFlipbook Object Reference"))))
  (return (`self.LastDirection`)))

(fn `UserConstructionScript`)